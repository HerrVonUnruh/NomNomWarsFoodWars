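; Player controller for a dice-driven board game that rolls the pawn and universal dice on Space or gamepad, and moves the mouse cursor by joystick.
; RollDice reads each result from the display name of the die's highest side component after a delay.
; Once both dice stop moving, it briefly shows the roll widget and enables unit movement.
; Key 1 toggles "Mikel Patch", a debug-style override that forces fixed results.
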(event Custom|Roll%20Dice
  (bind _universaldiceref (Variables|Default|GetuniversalDiceRef))
  (bind _pdiceref (Variables|Default|GetpDiceRef))
  (bind _dice_wp_ref (Variables|Default|GetDice_WP_Ref))
  (bind _pdiceref_2 (Variables|Default|GetpDiceRef))
  (bind _universaldiceref_2 (Variables|Default|GetuniversalDiceRef))
  (bind _returnvalue (Transformation|GetActorLocation _universaldiceref_2))
  (bind _returnvalue_2 (Transformation|GetActorLocation _pdiceref_2))
  (Variables|Default|SetCanRoll false)
  (Default|RollPawnDice _pdiceref)
  (Default|RollUniversalDice _universaldiceref)
  (if (not (Variables|Default|GetactivateMikelPatch))
    (Utilities|FlowControl|Delay 5.0)
    (Variables|Default|SetuHighest_ZAxis 1e+01)
    (Variables|Default|SetpHighest_ZAxis 1e+01)
    (for _array_element (Variables|/Game/Development/MainGame/BP_Universal_Dice.BP_Universal_Dice_C|GetuSideArr _universaldiceref)
      (if (< (Variables|Default|GetuHighest_ZAxis) (.z (Transformation|GetWorldLocation _array_element)))
        (Variables|Default|SetuHighest_ZAxis (.z (Transformation|GetWorldLocation _array_element)))
        (bind _output_get (Variables|Default|SetuTempStaticMesh _array_element))))
    (for _array_element_2 (Variables|/Game/Development/MainGame/BP_Pawn_Dice.BP_Pawn_Dice_C|GetpSideArr _pdiceref)
      (if (< (Variables|Default|GetpHighest_ZAxis) (.z (Transformation|GetWorldLocation _array_element_2)))
        (Variables|Default|SetpHighest_ZAxis (.z (Transformation|GetWorldLocation _array_element_2)))
        (bind _output_get_2 (Variables|Default|SetpTempStaticMesh _array_element_2))))
    ;[1 0 0 1 72] Universal/Red Dice
    (if (== (Utilities|String|GetCharacterasNumber (Utilities|GetDisplayName _output_get) 18) 49)
      (Variables|Default|SetResultUniversalDice 1)
      (Variables|Default|SetE_Universal_Dice_Results "NewEnumerator0")
      ;[0 0.07026 1 1 72] Pawn/BlueDice
      (if (== (Utilities|String|GetCharacterasNumber (Utilities|GetDisplayName _output_get_2) 13) 49) :!label _label
        (Variables|Default|SetResultPawnDice 1)
        (Variables|Default|SetE_Pawn_Dice_Results "NewEnumerator0")
        (Variables|Default|SetuDiceLocation _returnvalue_2 :!label _label_2)
        (Variables|Default|SetpDiceLocation _returnvalue)
        (Utilities|FlowControl|Delay 1.5)
        (if (and (Utilities|Operators|EqualEqual (Variables|Default|GetuDiceLocation) _returnvalue_2 0.0) (Utilities|Operators|EqualEqual (Variables|Default|GetpDiceLocation) _returnvalue 0.0))
          (Widget|SetVisibility (Variables|Default|GetDice_WP_Ref) "Visible")
          (Utilities|FlowControl|Sequence
            (:then_0
              (switch Utilities|FlowControl|Switch|SwitchonE_Universal_Dice_Results (Variables|Default|GetE_Universal_Dice_Results)
                (:NewEnumerator0
                  (Default|DisplayUniversalDiceRoll _dice_wp_ref "/Game/Art/Props/Dices/YannickConceptsDice1.YannickConceptsDice1"))
                (:NewEnumerator1
                  (Default|DisplayUniversalDiceRoll _dice_wp_ref "/Game/Art/Props/Dices/YannickConceptsDice2.YannickConceptsDice2"))
                (:NewEnumerator2
                  (Default|DisplayUniversalDiceRoll _dice_wp_ref "/Game/Art/Props/Dices/YannickConceptsDice3.YannickConceptsDice3"))
                (:NewEnumerator3
                  (Default|DisplayUniversalDiceRoll _dice_wp_ref "/Game/Art/Props/Dices/YannickConceptsDice4.YannickConceptsDice4"))
                (:NewEnumerator4
                  (Default|DisplayUniversalDiceRoll _dice_wp_ref "/Game/Art/Props/Dices/YannickConceptsDice5.YannickConceptsDice5"))
                (:NewEnumerator5
                  (Default|DisplayUniversalDiceRoll _dice_wp_ref "/Game/Art/Props/Dices/YannickConceptsDice6.YannickConceptsDice6"))))
            (:then_1
              (switch Utilities|FlowControl|Switch|SwitchonE_Pawn_Dice_Results (Variables|Default|GetE_Pawn_Dice_Results)
                (:NewEnumerator0
                  (Default|DisplayPawnDiceRoll _dice_wp_ref "/Game/Art/Props/Dices/YannickConceptsDice1.YannickConceptsDice1"))
                (:NewEnumerator1
                  (Default|DisplayPawnDiceRoll _dice_wp_ref "/Game/Art/Props/Dices/YannickConceptsDice2.YannickConceptsDice2"))
                (:NewEnumerator2
                  (Default|DisplayPawnDiceRoll _dice_wp_ref "/Game/Art/Props/Dices/YannickConceptsDice3.YannickConceptsDice3"))
                (:NewEnumerator3
                  (Default|DisplayPawnDiceRoll _dice_wp_ref "/Game/Art/Props/Dices/YannickConceptsDice4.YannickConceptsDice4"))
                (:NewEnumerator4
                  (Default|DisplayPawnDiceRoll _dice_wp_ref "/Game/Art/Props/Dices/YannickConceptsDice5.YannickConceptsDice5"))
                (:NewEnumerator5
                  (Default|DisplayPawnDiceRoll _dice_wp_ref "/Game/Art/Props/Dices/YannickConceptsDice6.YannickConceptsDice6")))))
          (Utilities|FlowControl|Delay 2.0)
          (Widget|SetVisibility _dice_wp_ref "Collapsed")
          (Utilities|Casting|CastToGamingInstance (Game|GetGameInstance))
          (Variables|Default|SetcanMoveUnits true)
          (Variables|Default|SetshowedWidget true)
          (else
            (goto _label_2)))
        (elif (== (Utilities|String|GetCharacterasNumber (Utilities|GetDisplayName _output_get_2) 13) 50)
          (Variables|Default|SetResultPawnDice 2)
          (Variables|Default|SetE_Pawn_Dice_Results "NewEnumerator1")
          (goto _label_2)
          (elif (== (Utilities|String|GetCharacterasNumber (Utilities|GetDisplayName _output_get_2) 13) 51)
            (Variables|Default|SetResultPawnDice 3)
            (Variables|Default|SetE_Pawn_Dice_Results "NewEnumerator2")
            (goto _label_2)
            (elif (== (Utilities|String|GetCharacterasNumber (Utilities|GetDisplayName _output_get_2) 13) 52)
              (Variables|Default|SetResultPawnDice 4)
              (Variables|Default|SetE_Pawn_Dice_Results "NewEnumerator3")
              (goto _label_2)
              (elif (== (Utilities|String|GetCharacterasNumber (Utilities|GetDisplayName _output_get_2) 13) 53)
                (Variables|Default|SetResultPawnDice 5)
                (Variables|Default|SetE_Pawn_Dice_Results "NewEnumerator4")
                (goto _label_2)
                (elif (== (Utilities|String|GetCharacterasNumber (Utilities|GetDisplayName _output_get_2) 13) 54)
                  (Variables|Default|SetResultPawnDice 6)
                  (Variables|Default|SetE_Pawn_Dice_Results "NewEnumerator5")
                  (goto _label_2)))))))
      (elif (== (Utilities|String|GetCharacterasNumber (Utilities|GetDisplayName _output_get) 18) 50)
        (Variables|Default|SetResultUniversalDice 2)
        (Variables|Default|SetE_Universal_Dice_Results "NewEnumerator1")
        (goto _label)
        (elif (== (Utilities|String|GetCharacterasNumber (Utilities|GetDisplayName _output_get) 18) 51)
          (Variables|Default|SetResultUniversalDice 3)
          (Variables|Default|SetE_Universal_Dice_Results "NewEnumerator2")
          (goto _label)
          (elif (== (Utilities|String|GetCharacterasNumber (Utilities|GetDisplayName _output_get) 18) 52)
            (Variables|Default|SetResultUniversalDice 4)
            (Variables|Default|SetE_Universal_Dice_Results "NewEnumerator3")
            (goto _label)
            (elif (== (Utilities|String|GetCharacterasNumber (Utilities|GetDisplayName _output_get) 18) 53)
              (Variables|Default|SetResultUniversalDice 5)
              (Variables|Default|SetE_Universal_Dice_Results "NewEnumerator4")
              (goto _label)
              (elif (== (Utilities|String|GetCharacterasNumber (Utilities|GetDisplayName _output_get) 18) 54)
                (Variables|Default|SetResultUniversalDice 6)
                (Variables|Default|SetE_Universal_Dice_Results "NewEnumerator5")
                (goto _label)))))))
    (else
      (Variables|Default|SetResultPawnDice 6)
      (Variables|Default|SetResultUniversalDice 16)
      (goto _label_2))))

(event Custom|MoveMouse
  (params (Delta :type Float%20%28double-precision%29))
  (bind (_locationx _locationy) (Game|Player|GetMousePosition))
  (bind _returnvalue (Input|AxisValues|GetJoyX))
  (bind _returnvalue_2 (Input|AxisValues|GetJoyY))
  (bind _sensitivity (Variables|Default|GetSensitivity))
  (bind _returnvalue_3 (Math|Vector2D|MakeVector2D _locationx _locationy))
  (bind _returnvalue_4 (Math|Vector2D|MakeVector2D _returnvalue _returnvalue_2))
  (bind _returnvalue_5 (* _returnvalue_4 _sensitivity))
  (bind _returnvalue_6 (* _returnvalue_5 Delta))
  (bind _returnvalue_7 (+ _returnvalue_3 _returnvalue_6))
  ;[1 1 1] MoveCursorWithJoystick
  (if (> (Math|Float|Absolute(Float) _returnvalue) 0.0)
    (Class|PlayerController|SetMouseLocation (Math|Float|Truncate (.x _returnvalue_7)) (Math|Float|Truncate (.y _returnvalue_7)))))

(event EventBeginPlay
  (bind _outactors (Actor|GetAllActorsOfClass "/Game/Development/MainGame/BP_Manager.BP_Manager_C"))
  (Variables|Default|SetManagerRef (Utilities|Array|Get(acopy) _outactors))
  (bind _outactors_2 (Actor|GetAllActorsOfClass "/Game/Development/MainGame/BP_Universal_Dice.BP_Universal_Dice_C"))
  (Variables|Default|SetuniversalDiceRef (Utilities|Array|Get(acopy) _outactors_2))
  (bind _outactors_3 (Actor|GetAllActorsOfClass "/Game/Development/MainGame/BP_Pawn_Dice.BP_Pawn_Dice_C"))
  (Variables|Default|SetpDiceRef (Utilities|Array|Get(acopy) _outactors_3))
  (bind _foundwidgets (Widget|GetAllWidgetsOfClass "/Game/Development/UI/WP_DiceRoll.WP_DiceRoll_C" true))
  (Variables|Default|SetDice_WP_Ref (Utilities|Array|Get(acopy) _foundwidgets))
  (bind _foundwidgets_2 (Widget|GetAllWidgetsOfClass "/Game/Development/UI/PlayerIndicator.PlayerIndicator_C" true))
  (Variables|Default|SetPlayer_Indicator_Ref (Utilities|Array|Get(acopy) _foundwidgets_2)))

(event EventTick
  (params (DeltaSeconds :type Float%20%28single-precision%29))
  (CallFunction|MoveMouse DeltaSeconds))

(event Input|KeyboardEvents|2
  (params (Key :type Key%20Structure :default "None")))

(event Input|KeyboardEvents|SpaceBar
  (params (Key :type Key%20Structure :default "None"))
  ;[1 1 1] Roll Dice
  (:Pressed
    (Variables|Default|SetshowedWidget false)
    (Variables|Default|SetcanMoveUnits false)
    (if (Variables|Default|GetCanRoll)
      (CallFunction|RollDice)
      (Audio|PlaySound2D "/Game/SoundDepartment/SFX/Dice_Rolling_v3.Dice_Rolling_v3" 1.0 1.0 0.0 0 0)
      (Utilities|FlowControl|Delay 8.2)
      (Widget|SetVisibility (Variables|/Game/Development/UI/PlayerIndicator.PlayerIndicator_C|GetPawn_Dice (Variables|Default|GetPlayer_Indicator_Ref)) "Visible"))))

(event Input|GamepadEvents|GamepadFaceButtonLeft
  (params (Key :type Key%20Structure :default "None"))
  ;[1 1 1] Roll Dice
  (:Pressed
    (Variables|Default|SetshowedWidget false)
    (Variables|Default|SetcanMoveUnits false)
    (if (Variables|Default|GetCanRoll)
      (CallFunction|RollDice)
      (Audio|PlaySound2D "/Game/SoundDepartment/SFX/Dice_Rolling_v3.Dice_Rolling_v3" 1.0 1.0 0.0 0 0)
      (Utilities|FlowControl|Delay 8.2)
      (Widget|SetVisibility (Variables|/Game/Development/UI/PlayerIndicator.PlayerIndicator_C|GetPawn_Dice (Variables|Default|GetPlayer_Indicator_Ref)) "Visible"))))

(event Input|KeyboardEvents|1
  (params (Key :type Key%20Structure :default "None"))
  ;[1 1 1] MIkel Patch
  (:Pressed
    (Utilities|FlowControl|FlipFlop
      (:A
        (Variables|Default|SetactivateMikelPatch true))
      (:B
        (Variables|Default|SetactivateMikelPatch false)))))

(fn ConstructionScript)

(fn SetupDiceandWidget
  (Variables|Default|SetbEnableClickEvents true)
  (Variables|Default|SetbShowMouseCursor true)
  (bind _outactors (Actor|GetAllActorsOfClass "/Game/Development/MainGame/BP_Universal_Dice.BP_Universal_Dice_C"))
  (Variables|Default|SetuniversalDiceRef (Utilities|Array|Get(acopy) _outactors))
  (bind _outactors_2 (Actor|GetAllActorsOfClass "/Game/Development/MainGame/BP_Pawn_Dice.BP_Pawn_Dice_C"))
  (Variables|Default|SetpDiceRef (Utilities|Array|Get(acopy) _outactors_2))
  (bind _returnvalue (UserInterface|CreateWidget "/Game/Development/UI/WP_DiceRoll.WP_DiceRoll_C"))
  (bind _output_get (Variables|Default|SetDice_WP_Ref _returnvalue))
  (UserInterface|Viewport|AddtoViewport _output_get 0)
  (Variables|Default|SetWP%20Universal%20Dice (Variables|/Game/Development/UI/WP_DiceRoll.WP_DiceRoll_C|GetWP_Universal_Dice (Variables|Default|GetDice_WP_Ref)))
  (Variables|Default|SetWP%20Pawn%20Dice (Variables|/Game/Development/UI/WP_DiceRoll.WP_DiceRoll_C|GetWP_Pawn_Dice (Variables|Default|GetDice_WP_Ref))))