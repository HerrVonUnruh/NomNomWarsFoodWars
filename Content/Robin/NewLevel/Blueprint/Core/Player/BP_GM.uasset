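; BP_GM, likely the game mode by its name, sets up a local multiplayer session on BeginPlay.
; It has the first BP_PC set up dice and widgets, then creates extra local players from the GamingInstance player count.
; It caches three player controllers regardless of count, shows a LoadingScreen widget and sets Game-and-UI input on the first controller.
; Input mapping and camera controller spawning nodes are present but never run.
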(event EventBeginPlay
  (bind _asbp_pc (Utilities|Casting|CastToBP_PC (Game|GetPlayerController 0)))
  (Default|SetupDiceandWidget _asbp_pc)
  (bind _asgaming_instance (Utilities|Casting|CastToGamingInstance (Game|GetGameInstance)))
  (bind _output_get (Variables|Default|SetNumb%20Of%20Players (Variables|/Game/Development/GamingInstance.GamingInstance_C|GetNumbOfPlayers _asgaming_instance)))
  (for _index (range 1 (- _output_get 1))
    (bind _output_get_2 (Variables|Default|SetIndex _index))
    (bind _returnvalue (Class|GameplayStatics|CreatePlayer _output_get_2)))
  (Variables|Default|SetArrPlayerControllers (Utilities|Array|MakeArray (Game|GetPlayerController 0) (Game|GetPlayerController 1) (Game|GetPlayerController 2)))
  (bind _returnvalue_2 (UserInterface|CreateWidget "/Game/Development/LoadingScreen.LoadingScreen_C" 0 false 0))
  (Variables|Default|SetisLoadingScreenOpen true)
  (UserInterface|Viewport|AddtoViewport _returnvalue_2 0)
  (Variables|Default|SetisLoadingScreenOpen false)
  (Input|SetInputModeGameandUI (Game|GetPlayerController 0) 0 "DoNotLock" true false))

(fn ConstructionScript)