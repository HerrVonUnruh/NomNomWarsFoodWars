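; Spell animation actor for the Wind Gust combat spell, visualizing gusts spreading from a target tile to the other attacked tiles.
; On play it reports a hit on the target tile, then spawns an animated gust per remaining tile, growing and facing outward at random speeds.
; Each finished gust reports its tile hit, and the spell completes when none remain.
; Construction tints three static meshes purple.
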(event Custom|OnShapeAnimationCompletedd
  (params (AnimatedShape :type BP%20Animated%20Wind%20Gust%20Object%20Reference))
  (bind _index (Variables|/Game/Robin/NewLevel/Blueprint/Core/CombatSetup/Spells/SpellAnimations/Components/BP_AnimatedWindGust.BP_AnimatedWindGust_C|GetIndex AnimatedShape))
  (bind _attackedindexes (Variables|Default|GetAttackedIndexes))
  (Default|CallOnSpellAnimationHitTile self _index)
  (Utilities|Array|RemoveItem _attackedindexes _index)
  (if (== (Utilities|Array|Length _attackedindexes) 0)
    (CallFunction|EventCompleteSpellAnimation)))

(event EventBeginPlay
  (|CallParentFunction) ; This node is disabled and will not be called.\nDrag off pins to build functionality.
)

(event Collision|EventActorBeginOverlap
  (params (OtherActor :type Actor%20Object%20Reference)))

(event EventTick
  (params (DeltaSeconds :type Float%20%28single-precision%29)))

(event EventEventPlaySpellAnimation
  (bind _targetindex (Variables|Default|GetTargetIndex))
  (bind _transform (CallFunction|GetTileTransform _targetindex))
  (Default|CallOnSpellAnimationHitTile self (Variables|Default|GetTargetIndex))
  (Utilities|Array|RemoveItem (Variables|Default|GetAttackedIndexes) (Variables|Default|GetTargetIndex))
  (for _array_element (Variables|Default|GetAttackedIndexes)
    (bind _returnvalue (Game|SpawnActorfromClass "/Game/Robin/NewLevel/Blueprint/Core/CombatSetup/Spells/SpellAnimations/Components/BP_AnimatedWindGust.BP_AnimatedWindGust_C" (Math|Transform|MakeTransform "0, 0, 0" "0, 0, 0" "1.000000,1.000000,1.000000") "AlwaysSpawn" "MultiplyWithRoot" 0 (Math|Transform|MakeTransform (.location _transform) (Math|Rotator|FindLookatRotation (.location _transform) (.location (CallFunction|GetTileTransform _array_element))) "0.500000,0.500000,0.500000") (Math|Transform|MakeTransform (.location (CallFunction|GetTileTransform _array_element)) (Math|Rotator|FindLookatRotation (.location _transform) (.location (CallFunction|GetTileTransform _array_element))) "1.200000,1.200000,1.200000") (Math|Random|RandomFloatinRange 0.8 1.5) _array_element 0))
    (EventDispatchers|BindEventtoOnShapeAnimationCompleted _returnvalue (delegate Custom|OnShapeAnimationCompletedd))))

(fn ConstructionScript
  (|CallParentFunction)
  (Rendering|Material|SetVectorParameterValueonMaterials (Variables|Default|GetStaticMeshOne) "Color" (Math|Conversions|ToVector(LinearColor) "(R=0.258824,G=0.019608,B=0.635294,A=1.000000)"))
  (Rendering|Material|SetVectorParameterValueonMaterials (Variables|Default|GetStaticMeshOne1) "Color" (Math|Conversions|ToVector(LinearColor) "(R=0.405798,G=0.028985,B=1.000000,A=1.000000)"))
  (Rendering|Material|SetVectorParameterValueonMaterials (Variables|Default|GetStaticMeshOne2) "Color" (Math|Conversions|ToVector(LinearColor) "(R=0.258824,G=0.019608,B=0.635294,A=1.000000)")))