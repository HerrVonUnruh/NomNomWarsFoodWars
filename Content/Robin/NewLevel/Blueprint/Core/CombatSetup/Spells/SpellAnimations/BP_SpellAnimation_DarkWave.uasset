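; Spell animation actor for Dark Wave, a purple three-mesh effect played on the target tile.
; On play it moves to the target tile, and a timeline drives the effect's scale and material opacity before signalling completion.
; Once playback passes an early threshold, a DoOnce fires the tile-hit callback once per attacked index, passing the target index each time rather than the looped one.
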(event EventBeginPlay
  (|CallParentFunction) ; This node is disabled and will not be called.\nDrag off pins to build functionality.
)

(event Collision|EventActorBeginOverlap
  (params (OtherActor :type Actor%20Object%20Reference)))

(event EventTick
  (params (DeltaSeconds :type Float%20%28single-precision%29)))

(event EventEventPlaySpellAnimation
  (Transformation|SetActorLocation (.location (CallFunction|GetTileTransform (Variables|Default|GetTargetIndex))) false false)
  (bind (_direction _opacity _scale) (Timeline|Timeline_DarkWave PlayFromStart)
    (:Update
      (Transformation|SetRelativeScale3D (Variables|Default|GetAnim_Scale) _scale)
      (Rendering|Material|SetScalarParameterValueonMaterials (Variables|Default|GetStaticMeshOne) "Opacity" _opacity)
      (if (>= (Components|Timeline|GetPlaybackPosition (Variables|Default|GetTimeline_DarkWave)) 0.2)
        (Utilities|FlowControl|DoOnce false
          (:Completed
            (for _array_element (Variables|Default|GetAttackedIndexes)
              (Default|CallOnSpellAnimationHitTile self (Variables|Default|GetTargetIndex)))))))
    (:Finished
      (CallFunction|EventCompleteSpellAnimation))))

(fn ConstructionScript
  (|CallParentFunction)
  (Rendering|Material|SetVectorParameterValueonMaterials (Variables|Default|GetStaticMeshOne) "Color" (Math|Conversions|ToVector(LinearColor) "(R=0.258824,G=0.019608,B=0.635294,A=1.000000)"))
  (Rendering|Material|SetVectorParameterValueonMaterials (Variables|Default|GetStaticMeshOne1) "Color" (Math|Conversions|ToVector(LinearColor) "(R=0.405798,G=0.028985,B=1.000000,A=1.000000)"))
  (Rendering|Material|SetVectorParameterValueonMaterials (Variables|Default|GetStaticMeshOne2) "Color" (Math|Conversions|ToVector(LinearColor) "(R=0.258824,G=0.019608,B=0.635294,A=1.000000)")))