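; Spell animation actor for a slime ball thrown from an origin tile to a target tile in tile-based combat.
; A timeline drives a slerped path with height offset, plus scale and opacity on three nested meshes tinted green in construction.
; Past a playback threshold it fires the hit callback once per attacked index, always passing the target index.
; The timeline's end completes the spell animation.
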(event EventBeginPlay
  (|CallParentFunction) ; This node is disabled and will not be called.\nDrag off pins to build functionality.
)

(event Collision|EventActorBeginOverlap
  (params (OtherActor :type Actor%20Object%20Reference)))

(event EventTick
  (params (DeltaSeconds :type Float%20%28single-precision%29)))

(event EventEventPlaySpellAnimation
  (Transformation|SetActorLocation (.location (CallFunction|GetTileTransform (Variables|Default|GetTargetIndex))) false false)
  (bind (_direction _locationalpha _locationz _opacity _scale) (Timeline|Timeline_SlimeBall PlayFromStart)
    (:Update
      (Transformation|SetActorLocation (+ (Class|KismetMathLibrary|VectorSlerpNormals (.location (CallFunction|GetTileTransform (Variables|Default|GetOriginIndex))) (.location (CallFunction|GetTileTransform (Variables|Default|GetTargetIndex))) _locationalpha) (Math|Vector|MakeVector 0.0 0.0 _locationz)) false false)
      (Rendering|Material|SetScalarParameterValueonMaterials (Variables|Default|GetStaticMeshOneInner) "Opacity" _opacity)
      (Transformation|SetRelativeScale3D (Variables|Default|GetAnim_Scale) _scale)
      (if (>= (Components|Timeline|GetPlaybackPosition (Variables|Default|GetTimeline_SlimeBall)) 0.55)
        (Utilities|FlowControl|DoOnce false
          (:Completed
            (for _array_element (Variables|Default|GetAttackedIndexes)
              (Default|CallOnSpellAnimationHitTile self (Variables|Default|GetTargetIndex)))))))
    (:Finished
      (CallFunction|EventCompleteSpellAnimation))))

(fn ConstructionScript
  (|CallParentFunction)
  (Rendering|Material|SetVectorParameterValueonMaterials (Variables|Default|GetStaticMeshOneInner) "Color" (Math|Conversions|ToVector(LinearColor) "(R=0.541394,G=0.723958,B=0.475212,A=1.000000)"))
  (Rendering|Material|SetVectorParameterValueonMaterials (Variables|Default|GetStaticMeshOneMiddle) "Color" (Math|Conversions|ToVector(LinearColor) "(R=0.347005,G=0.812500,B=0.380256,A=1.000000)"))
  (Rendering|Material|SetVectorParameterValueonMaterials (Variables|Default|GetStaticMeshOneOutside) "Color" (Math|Conversions|ToVector(LinearColor) "(R=0.129015,G=0.427083,B=0.149650,A=1.000000)")))