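; Combat action for grid-based unit movement that shows reachable tiles and the path to the hovered tile, then moves the selected unit along it.
; Two grid pathfinders run time-sliced searches limited by the unit's movement points, diagonal rule and valid tile types, and their completion events set tile states.
; Hovering another unit previews its reach, executing passes the path to the combat system, and walking events pause highlighting until movement ends.
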(event EventBeginPlay
  (bind _playeractions (Variables|Default|GetPlayerActions))
  (bind _selectedunit (Variables|/Game/Robin/NewLevel/Blueprint/Core/Player/BP_PlayerActions.BP_PlayerActions_C|GetSelectedUnit _playeractions))
  (|CallParentFunction)
  (EventDispatchers|BindEventtoOnPathfindingCompleted (Variables|/Game/Robin/NewLevel/Blueprint/Grid/BP_Grid.BP_Grid_C|GetGridPathfinding_Reachables (Variables|/Game/Robin/NewLevel/Blueprint/Core/Player/BP_PlayerActions.BP_PlayerActions_C|GetGrid (Variables|Default|GetPlayerActions))) (EventDispatchers|CreateEvent :!event OnPathfindingCompletedReachables))
  (EventDispatchers|BindEventtoOnPathfindingCompleted (Variables|/Game/Robin/NewLevel/Blueprint/Grid/BP_Grid.BP_Grid_C|GetGrid%20Pathfinding (Variables|/Game/Robin/NewLevel/Blueprint/Core/Player/BP_PlayerActions.BP_PlayerActions_C|GetGrid (Variables|Default|GetPlayerActions))) (EventDispatchers|CreateEvent :!event OnPathfindingCompletedPath))
  (EventDispatchers|BindEventtoOnUnitStartedWalking _selectedunit (EventDispatchers|CreateEvent :!event OnUnitStartedWalking))
  (EventDispatchers|BindEventtoOnUnitFinishedWalking _selectedunit (EventDispatchers|CreateEvent :!event OnUnitFinishedWalking))
  (CallFunction|GenerateReachable (Variables|/Game/Robin/NewLevel/Blueprint/Core/Player/BP_PlayerActions.BP_PlayerActions_C|GetSelectedUnit (Variables|Default|GetPlayerActions))))

(event Collision|EventActorBeginOverlap
  (params (OtherActor :type Actor%20Object%20Reference))
  (|CallParentFunction OtherActor) ; This node is disabled and will not be called.\nDrag off pins to build functionality.
)

(event EventTick
  (params (DeltaSeconds :type Float%20%28single-precision%29))
  (|CallParentFunction DeltaSeconds) ; This node is disabled and will not be called.\nDrag off pins to build functionality.
)

(event EventEndPlay
  (params (EndPlayReason :type EEndPlayReason%20Enum :default "Destroyed"))
  (bind _playeractions (Variables|Default|GetPlayerActions))
  (bind _grid (Variables|/Game/Robin/NewLevel/Blueprint/Core/Player/BP_PlayerActions.BP_PlayerActions_C|GetGrid _playeractions))
  (|CallParentFunction EndPlayReason)
  (Default|ClearStatefromTiles _grid "NewEnumerator7")
  (Default|ClearStatefromTiles _grid "NewEnumerator4"))

(fn ConstructionScript
  (|CallParentFunction))

(fn GenerateReachable
  (params (Unit :type BP%20Unit%20Object%20Reference))
  (if (!= Unit (Variables|Default|GetCurrentUnitForReachables))
    (Variables|Default|SetCurrentUnitForReachables Unit)
    (Default|ClearStatefromTiles (Variables|/Game/Robin/NewLevel/Blueprint/Core/Player/BP_PlayerActions.BP_PlayerActions_C|GetGrid (Variables|Default|GetPlayerActions)) "NewEnumerator7")
    (Default|FindPath (Variables|/Game/Robin/NewLevel/Blueprint/Grid/BP_Grid.BP_Grid_C|GetGridPathfinding_Reachables (Variables|/Game/Robin/NewLevel/Blueprint/Core/Player/BP_PlayerActions.BP_PlayerActions_C|GetGrid (Variables|Default|GetPlayerActions))) (Variables|/Game/Robin/NewLevel/Blueprint/Core/Units/BP_Unit.BP_Unit_C|GetIndex (Variables|Default|GetCurrentUnitForReachables)) (Utilities|Struct|MakeIntPoint -999 -999) (.CanMoveDiagonally (Utilities|Struct|BreakS_UnitData_Stats (Utilities|Struct|BreakS_UnitData (Variables|/Game/Robin/NewLevel/Blueprint/Core/Units/BP_Unit.BP_Unit_C|GetUnitData (Variables|Default|GetCurrentUnitForReachables))))) (.ValidTileTypes (Utilities|Struct|BreakS_UnitData_Stats (Utilities|Struct|BreakS_UnitData (Variables|/Game/Robin/NewLevel/Blueprint/Core/Units/BP_Unit.BP_Unit_C|GetUnitData (Variables|Default|GetCurrentUnitForReachables))))) 0.1 0.25 true (.MP_Current (Utilities|Struct|BreakS_UnitData_Stats (Utilities|Struct|BreakS_UnitData (Variables|/Game/Robin/NewLevel/Blueprint/Core/Units/BP_Unit.BP_Unit_C|GetUnitData (Variables|Default|GetCurrentUnitForReachables))))))))

(fn OnPathfindingCompletedReachables
  (params (Reachables :type Array%20of%20Int%20Point%20Structures))
  (if (not (Variables|Default|GetIsUnitWalking))
    (for _array_element Reachables
      (Default|AddStatetoTile (Variables|/Game/Robin/NewLevel/Blueprint/Core/Player/BP_PlayerActions.BP_PlayerActions_C|GetGrid (Variables|Default|GetPlayerActions)) _array_element "NewEnumerator7"))))

(fn ExecuteHoweredAction
  (params (Index :type Int%20Point%20Structure))
  (bind _playeractions (Variables|Default|GetPlayerActions))
  (bind _hoveredunit (Variables|/Game/Robin/NewLevel/Blueprint/Core/Player/BP_PlayerActions.BP_PlayerActions_C|GetHoveredUnit _playeractions))
  (|CallParentFunction Index)
  (if (not (Variables|Default|GetIsUnitWalking))
    (Utilities|IsValid _hoveredunit
      (:Is%20Valid
        (CallFunction|GenerateReachable _hoveredunit))
      (:Is%20Not%20Valid
        (CallFunction|GenerateReachable (Variables|/Game/Robin/NewLevel/Blueprint/Core/Player/BP_PlayerActions.BP_PlayerActions_C|GetSelectedUnit _playeractions))
        (CallFunction|GeneratePath)))))

(fn GeneratePath
  (bind _playeractions (Variables|Default|GetPlayerActions))
  (bind _selectedunit (Variables|/Game/Robin/NewLevel/Blueprint/Core/Player/BP_PlayerActions.BP_PlayerActions_C|GetSelectedUnit _playeractions))
  (bind _unitdata (Variables|/Game/Robin/NewLevel/Blueprint/Core/Units/BP_Unit.BP_Unit_C|GetUnitData _selectedunit))
  (bind _stats (Utilities|Struct|BreakS_UnitData _unitdata))
  (bind (_validtiletypes _canmovediagonally _mp_current) (Utilities|Struct|BreakS_UnitData_Stats _stats))
  (Default|ClearStatefromTiles (Variables|/Game/Robin/NewLevel/Blueprint/Core/Player/BP_PlayerActions.BP_PlayerActions_C|GetGrid (Variables|Default|GetPlayerActions)) "NewEnumerator4")
  (Utilities|Array|Clear (Variables|Default|GetGeneratedPath))
  (Default|FindPath (Variables|/Game/Robin/NewLevel/Blueprint/Grid/BP_Grid.BP_Grid_C|GetGrid%20Pathfinding (Variables|/Game/Robin/NewLevel/Blueprint/Core/Player/BP_PlayerActions.BP_PlayerActions_C|GetGrid (Variables|Default|GetPlayerActions))) (Variables|/Game/Robin/NewLevel/Blueprint/Core/Units/BP_Unit.BP_Unit_C|GetIndex _selectedunit) (Variables|/Game/Robin/NewLevel/Blueprint/Core/Player/BP_PlayerActions.BP_PlayerActions_C|GetHowered%20Tile (Variables|Default|GetPlayerActions)) _canmovediagonally _validtiletypes 0.1 0.15 false _mp_current))

(fn OnPathfindingCompletedPath
  (params (Path :type Array%20of%20Int%20Point%20Structures))
  (bind _output_get (Variables|Default|SetGeneratedPath Path))
  (for _array_element _output_get
    (Default|AddStatetoTile (Variables|/Game/Robin/NewLevel/Blueprint/Core/Player/BP_PlayerActions.BP_PlayerActions_C|GetGrid (Variables|Default|GetPlayerActions)) _array_element "NewEnumerator4")))

(fn ExecuteAction
  (params (Index :type Int%20Point%20Structure))
  (bind _playeractions (Variables|Default|GetPlayerActions))
  (|CallParentFunction Index)
  (if (> (Utilities|Array|Length (Variables|Default|GetGeneratedPath)) 0)
    (Default|MoveUnit (Variables|/Game/Robin/NewLevel/Blueprint/Core/Player/BP_PlayerActions.BP_PlayerActions_C|GetCombatSystem _playeractions) (Variables|/Game/Robin/NewLevel/Blueprint/Core/Player/BP_PlayerActions.BP_PlayerActions_C|GetSelectedUnit _playeractions) (Variables|Default|GetGeneratedPath))
    (Utilities|Array|Clear (Variables|Default|GetGeneratedPath))))

(fn OnUnitStartedWalking
  (params (Unit :type BP%20Unit%20Object%20Reference))
  (Variables|Default|SetIsUnitWalking true)
  (Default|ClearStatefromTiles (Variables|/Game/Robin/NewLevel/Blueprint/Core/Player/BP_PlayerActions.BP_PlayerActions_C|GetGrid (Variables|Default|GetPlayerActions)) "NewEnumerator7")
  (Variables|Default|SetCurrentUnitForReachables 0))

(fn OnUnitFinishedWalking
  (params (Unit :type BP%20Unit%20Object%20Reference))
  (Variables|Default|SetIsUnitWalking false)
  (CallFunction|ExecuteAction (Variables|/Game/Robin/NewLevel/Blueprint/Core/Player/BP_PlayerActions.BP_PlayerActions_C|GetHowered%20Tile (Variables|Default|GetPlayerActions))))