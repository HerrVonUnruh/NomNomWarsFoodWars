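; Match manager for a turn-based, dice and grid game of up to three players, handling turns, respawns, pause and game over.
; Init caches scene actors, widgets and GamingInstance settings, then grants optional KingKiller tokens.
; A Delay-based loop runs the turn timer; expiry or SwitchTurnBUTTON rotates players through CameraController, resets dice and respawns that team's dead units, killing spawn-tile occupants.
; Game over disables input and plays the winning faction's video.
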(event Custom|Pawn%20hast%20been%20settet
  ;[0 0.09648 1 1 72] Turn&Game Events
  (Variables|Default|SetPawn%20has%20been%20set true))

(event Custom|WinConditionFullfilled
  ;[0 0.09648 1 1 72] Turn&Game Events
  (Variables|Default|SetGameOver true))

(event Custom|New%20Turn
  ;[0 0.09648 1 1 72] Turn&Game Events
  (Variables|Default|SetPawn%20has%20been%20set false))

(event Custom|GameIsOver
  ;[0 0.0366 1 1 72] Game Over
  (Input|DisableInput (Game|Player|GetPlayerPawn 0) (Game|GetPlayerController 0))
  (Variables|Default|SetGameOver true)
  (bind _returnvalue (CallFunction|GetPlayerID (.cameraController (Variables|Default|GetcameraController))))
  (if (== _returnvalue 1)
    (Variables|Default|SetPlayer1Won true)
    (Utilities|FlowControl|Delay 1.0)
    (bind _asgaming_instance (Utilities|Casting|CastToGamingInstance (Game|GetGameInstance)))
    (if (Utilities|Enum|Equal(Enum) (Utilities|Text|ToText(String) (Variables|/Game/Development/GamingInstance.GamingInstance_C|GetPlayerOne _asgaming_instance)) (Variables|Default|GetFastFoodNation))
      (bind _returnvalue_2 (UserInterface|CreateWidget "/Game/Videos/WinnigVideo.WinnigVideo_C" 0 "/Game/Videos/MP_Video.MP_Video" (Variables|Default|GetMediaSound) :!label _label))
      (UserInterface|Viewport|AddtoViewport _returnvalue_2 0)
      (CameraShake|Start (Variables|Default|GetMediaSound))
      (Utilities|FlowControl|Delay 7.0)
      (Widget|RemovefromParent _returnvalue_2)
      (else
        (bind _asgaming_instance_2 (Utilities|Casting|CastToGamingInstance (Game|GetGameInstance)))
        (if (Utilities|Enum|Equal(Enum) (Utilities|Text|ToText(String) (Variables|/Game/Development/GamingInstance.GamingInstance_C|GetPlayerOne _asgaming_instance_2)) (Variables|Default|GetFruityZone))
          (bind _returnvalue_3 (UserInterface|CreateWidget "/Game/Videos/WinnigVideo.WinnigVideo_C" 0 "/Game/Videos/MP_Video.MP_Video" (Variables|Default|GetMediaSound) :!label _label_2))
          (UserInterface|Viewport|AddtoViewport _returnvalue_3 0)
          (CameraShake|Start (Variables|Default|GetMediaSound))
          (Utilities|FlowControl|Delay 11.5)
          (Widget|RemovefromParent _returnvalue_3)
          (else
            (bind _asgaming_instance_3 (Utilities|Casting|CastToGamingInstance (Game|GetGameInstance)))
            (if (Utilities|Enum|Equal(Enum) (Utilities|Text|ToText(String) (Variables|/Game/Development/GamingInstance.GamingInstance_C|GetPlayerOne _asgaming_instance_3)) (Variables|Default|GetCandyLand))
              (bind _returnvalue_4 (UserInterface|CreateWidget "/Game/Videos/WinnigVideo.WinnigVideo_C" 0 "/Game/Videos/MP_Video.MP_Video" (Variables|Default|GetMediaSound) :!label _label_3))
              (UserInterface|Viewport|AddtoViewport _returnvalue_4 0)
              (CameraShake|Start (Variables|Default|GetMediaSound))
              (Utilities|FlowControl|Delay 7.0)
              (Widget|RemovefromParent _returnvalue_4))))))
    (elif (== _returnvalue 2)
      (Variables|Default|SetPlayer2Won true)
      (Utilities|FlowControl|Delay 1.0)
      (bind _asgaming_instance_4 (Utilities|Casting|CastToGamingInstance (Game|GetGameInstance)))
      (if (Utilities|Enum|Equal(Enum) (Utilities|Text|ToText(String) (Variables|/Game/Development/GamingInstance.GamingInstance_C|GetPlayerTwo _asgaming_instance_4)) (Variables|Default|GetFastFoodNation))
        (goto _label)
        (else
          (bind _asgaming_instance_5 (Utilities|Casting|CastToGamingInstance (Game|GetGameInstance)))
          (if (Utilities|Enum|Equal(Enum) (Utilities|Text|ToText(String) (Variables|/Game/Development/GamingInstance.GamingInstance_C|GetPlayerTwo _asgaming_instance_5)) (Variables|Default|GetFruityZone))
            (goto _label_2)
            (else
              (bind _asgaming_instance_6 (Utilities|Casting|CastToGamingInstance (Game|GetGameInstance)))
              (if (Utilities|Enum|Equal(Enum) (Utilities|Text|ToText(String) (Variables|/Game/Development/GamingInstance.GamingInstance_C|GetPlayerTwo _asgaming_instance_6)) (Variables|Default|GetCandyLand))
                (goto _label_3))))))
      (elif (== _returnvalue 3)
        (Variables|Default|SetPlayer3Won true)
        (Utilities|FlowControl|Delay 1.0)
        (bind _asgaming_instance_7 (Utilities|Casting|CastToGamingInstance (Game|GetGameInstance)))
        (if (Utilities|Enum|Equal(Enum) (Utilities|Text|ToText(String) (Variables|/Game/Development/GamingInstance.GamingInstance_C|GetPlayerThree _asgaming_instance_7)) (Variables|Default|GetFastFoodNation))
          (goto _label)
          (else
            (bind _asgaming_instance_8 (Utilities|Casting|CastToGamingInstance (Game|GetGameInstance)))
            (if (Utilities|Enum|Equal(Enum) (Utilities|Text|ToText(String) (Variables|/Game/Development/GamingInstance.GamingInstance_C|GetPlayerThree _asgaming_instance_8)) (Variables|Default|GetFruityZone))
              (goto _label_2)
              (else
                (bind _asgaming_instance_9 (Utilities|Casting|CastToGamingInstance (Game|GetGameInstance)))
                (if (Utilities|Enum|Equal(Enum) (Utilities|Text|ToText(String) (Variables|/Game/Development/GamingInstance.GamingInstance_C|GetPlayerThree _asgaming_instance_9)) (Variables|Default|GetCandyLand))
                  (goto _label_3))))))))))

(event Custom|AllUnitsHaveBeenSet
  ;[0 0.09648 1 1 72] Turn&Game Events
  (Variables|Default|SetAllUnitsSet true))

(event Custom|CameraShake
  ;[0 1 0.9843 1 72] CameraShake
  (Camera|PlayWorldCameraShake "/Game/Robin/BP_CameraShake.BP_CameraShake_C" (Transformation|GetWorldLocation (Variables|Default|GetCamera (.cameraController (Variables|Default|GetcameraController)))) 0.0 5e+02))

(event Custom|VFX_Timer
  ;[0 1 0.1112 1 72] VFX Timer
  (Utilities|FlowControl|Delay 0.5)
  (Components|Activation|Deactivate (Variables|Default|GetVFX_RespawnGreen)))

(event EventBeginPlay
  ;[1 0.0344 0 1 200] Core Begin Play
  (Utilities|FlowControl|Delay 2.0)
  (bind _foundwidgets (CallFunction|InitGame))
  ;;[1 1 1] Checks if the PlayerUI Widget != null
  (if (>= (Utilities|Array|Length _foundwidgets) 1)
    _
    (else
      (Utilities|FlowControl|Delay 1e+01)
      (CallFunction|ResetUpPlayerUiifFailed)))
  (CallFunction|SetKingKilllerTokens)
  (Variables|Default|SetplayerTxt "Player 1")
  (Utilities|FlowControl|Delay 3.0)
  (Variables|Default|SetshowTxt false)
  (CallFunction|TurnTimer :!label _label)
  (if (Variables|Default|GetNew%20Turn%20Begins)
    (Variables|Default|SetNew%20Turn%20Begins false)
    (CallFunction|ResetDiceResults)
    (if (not (Variables|Default|GetGameOver))
      (Variables|Default|SetturnDone false)
      (Variables|Default|SetAllUnitsSet false)
      (Variables|Default|SetPawn%20has%20been%20set false)
      (CallFunction|SwitchPlayerTurn (.cameraController (Variables|Default|GetcameraController)))
      (CallFunction|ResetKingKillerTokenCheck)
      (CallFunction|GetPlayerID (.cameraController (Variables|Default|GetcameraController)))
      (CallFunction|CheckWhichPlayerTurnItIs)
      (Utilities|FlowControl|Delay 3.0)
      (Variables|Default|SetshowTxt false)
      (Default|ShowPlayerID (Variables|Default|GetPlayerNumberUI))
      (Variables|Default|Settime (Variables|Default|GettimeRef))
      (bind _asbp_pc (Utilities|Casting|CastToBP_PC (Game|GetPlayerController 0)))
      (Variables|/Game/Robin/NewLevel/Blueprint/Core/Player/BP_PC.BP_PC_C|SetshowedWidget _asbp_pc false)
      (CallFunction|HandleUnitRespawn)
      (goto _label))
    (else
      (Utilities|FlowControl|Delay 1.0)
      (goto _label))))

(event Input|ActionEvents|InputActionPauseGame
  (params (Key :type Key%20Structure :default "None"))
  ;[1 0 0 1 72] IA_PauseMenu
  (:Pressed
    (bind _asbp_gm (Utilities|Casting|CastToBP_GM (Game|GetGameMode)))
    (if (not (Variables|/Game/Robin/NewLevel/Blueprint/Core/Player/BP_GM.BP_GM_C|GetisLoadingScreenOpen _asbp_gm))
      (if (Variables|Default|GetisPauseMenuOpen)
        (Widget|SetVisibility (Variables|Default|GetpauseMenuRef) "Collapsed")
        (Input|SetInputModeGameandUI (Game|GetPlayerController 0) 0 "DoNotLock" true false)
        (Variables|Default|SetisPauseMenuOpen false)
        (Game|SetGamePaused false)
        (else
          (Variables|Default|SetisPauseMenuOpen true)
          (Widget|SetVisibility (Variables|Default|GetpauseMenuRef) "Visible")
          (Game|SetGamePaused true)
          (Input|SetInputModeGameandUI (Game|GetPlayerController 0) (Variables|Default|GetpauseMenuRef) "DoNotLock" true false))))))

(fn ConstructionScript)

(fn Timer
  (bind _asbp_pc (Utilities|Casting|CastToBP_PC (Game|GetPlayerController 0)))
  (if (Variables|/Game/Robin/NewLevel/Blueprint/Core/Player/BP_PC.BP_PC_C|GetshowedWidget _asbp_pc)
    (if (> (Variables|Default|Gettime) 0.0)
      (bind _output_get (Variables|Default|Settime (- (Variables|Default|Gettime) 1.0)))
      (if (<= _output_get 1e+01)
        (Audio|PlaySound2D "/Game/SoundDepartment/SFX/CooleSoundEffekt/SFX_Timer_Running_Out.SFX_Timer_Running_Out" 1.0 1.0 0.0 0 0))
      (return _output_get)
      (else
        (Variables|Default|SetNew%20Turn%20Begins true)
        (Variables|Default|SetPawn%20has%20been%20set false)
        (Variables|Default|SetturnDone false)
        (return 0.0)))
    (else
      (return (Variables|Default|Gettime)))))

(fn SwitchTurnBUTTON
  (Variables|Default|SetNew%20Turn%20Begins true)
  (Variables|Default|SetNew%20Turn%20Begins false)
  (CallFunction|ResetDiceResults)
  (if (not (Variables|Default|GetGameOver))
    (Variables|Default|SetturnDone false)
    (Variables|Default|SetAllUnitsSet false)
    (Variables|Default|SetPawn%20has%20been%20set false)
    (CallFunction|SwitchPlayerTurn (.cameraController (Variables|Default|GetcameraController)))
    (CallFunction|ResetKingKillerTokenCheck)
    (bind _returnvalue (CallFunction|GetPlayerID (.cameraController (Variables|Default|GetcameraController))))
    (CallFunction|CheckWhichPlayerTurnItIs _returnvalue _returnvalue _returnvalue)
    (Variables|Default|SetshowTxt false)
    (Default|ShowPlayerID (Variables|Default|GetPlayerNumberUI))
    (Variables|Default|Settime (Variables|Default|GettimeRef))
    (bind _asgaming_instance (Utilities|Casting|CastToGamingInstance (Game|GetGameInstance)))
    (bind _asbp_pc (Utilities|Casting|CastToBP_PC (Game|GetPlayerController (Variables|/Game/Development/GamingInstance.GamingInstance_C|GetplayerIndex _asgaming_instance))))
    (Variables|/Game/Robin/NewLevel/Blueprint/Core/Player/BP_PC.BP_PC_C|SetshowedWidget _asbp_pc false)
    (CallFunction|HandleUnitRespawn)))

(fn RespawnUnit
  (params (Unit :type BP%20Unit%20Object%20Reference) (UnitCopy :type BP%20Unit%20Object%20Reference) (index :type Integer))
  (LocalVariables|Set_unit Unit)
  (bind _returnvalue (CallFunction|ComparePlayerNumandTeamIndex (LocalVariables|Get_unit)))
  (if _returnvalue
    (CallFunction|HandleVFX (Class|KismetMathLibrary|ToInt64(Integer) (Variables|/Game/Robin/NewLevel/Blueprint/Core/Units/BP_Unit.BP_Unit_C|GetTeamIndex (LocalVariables|Get_unit))) (LocalVariables|Get_unit))
    (CallFunction|PlaceUnitatSpawn (LocalVariables|Get_unit))
    (else
      (Variables|/Game/Robin/NewLevel/Blueprint/Core/Units/BP_Unit.BP_Unit_C|SetwaitForRespawn (LocalVariables|Get_unit) false))))

(fn SafeKingKillerTokens
  (params (index :type Integer) (tokenValue :type Integer))
  (if (== index 1)
    (Variables|/Game/Development/GamingInstance.GamingInstance_C|SettokenPlayer1 (Variables|Default|GetAs%20Gaming%20Instance) tokenValue)
    (elif (== index 2)
      (Variables|/Game/Development/GamingInstance.GamingInstance_C|SettokensPlayer2 (Variables|Default|GetAs%20Gaming%20Instance) tokenValue)
      (elif (== index 3)
        (Variables|/Game/Development/GamingInstance.GamingInstance_C|SettokensPlayer3 (Variables|Default|GetAs%20Gaming%20Instance) tokenValue)))))

(fn ComparePlayerNumandTeamIndex
  (params (unit :type BP%20Unit%20Object%20Reference))
  (bind _returnvalue (CallFunction|GetPlayerID (.cameraController (Variables|Default|GetcameraController))))
  (return (== _returnvalue (Variables|/Game/Robin/NewLevel/Blueprint/Core/Units/BP_Unit.BP_Unit_C|GetTeamIndex unit))))

(fn PlaceUnitatSpawn
  (params (unit :type BP%20Unit%20Object%20Reference))
  (LocalVariables|SetunitToPlace unit)
  (Variables|/Game/Robin/NewLevel/Blueprint/Core/Units/BP_Unit.BP_Unit_C|SetisDead (LocalVariables|GetunitToPlace) false)
  (CallFunction|CheckifUnitIsonTile (Variables|/Game/Robin/NewLevel/Blueprint/Core/Units/BP_Unit.BP_Unit_C|GetSpawnPoint (LocalVariables|GetunitToPlace)))
  (Variables|/Game/Robin/NewLevel/Blueprint/Core/Units/BP_Unit.BP_Unit_C|SetTeamIndex (LocalVariables|GetunitToPlace) (Variables|/Game/Robin/NewLevel/Blueprint/Core/Units/BP_Unit.BP_Unit_C|GetteamIndexRef (LocalVariables|GetunitToPlace)))
  (Default|SetUnitIndexonGrid (Variables|Default|GetcombatSystem) (LocalVariables|GetunitToPlace) (Variables|/Game/Robin/NewLevel/Blueprint/Core/Units/BP_Unit.BP_Unit_C|GetSpawnPoint (LocalVariables|GetunitToPlace)) false false)
  (Transformation|SetActorRotation (LocalVariables|GetunitToPlace) (Variables|/Game/Robin/NewLevel/Blueprint/Core/Units/BP_Unit.BP_Unit_C|GetSpawnRotation (LocalVariables|GetunitToPlace)))
  (Default|SetAnimationState (LocalVariables|GetunitToPlace) "NewEnumerator0")
  (Default|SetCurrentHP (LocalVariables|GetunitToPlace) 50)
  (Utilities|Array|RemoveItem (Variables|/Game/Development/MainGame/UnitSpawner.UnitSpawner_C|GetdeadUnits (Variables|Default|GetspawnerRef)) (LocalVariables|GetunitToPlace))
  (if (Utilities|Enum|Equal(Enum) (Variables|/Game/Robin/NewLevel/Blueprint/Core/Units/BP_Unit.BP_Unit_C|GetUnitType (LocalVariables|GetunitToPlace)) "NewEnumerator4")
    (Audio|PlaySound2D "/Game/SoundDepartment/SFX/Marshmallow_Soldier_voicedselect_unit_v3_lol.Marshmallow_Soldier_voicedselect_unit_v3_lol" 1.0 1.0 0.0 0 0)))

(fn SetUpGameValues
  (bind _winmanager (Variables|Default|GetwinManager))
  (bind _foundwidgets (Widget|GetAllWidgetsOfClass "/Game/Development/UI/WP_PauseMenu.WP_PauseMenu_C" true))
  (Variables|Default|SetpauseMenuRef (Utilities|Array|Get(acopy) _foundwidgets))
  (bind _outactors (Actor|GetAllActorsOfClass "/Game/Robin/NewLevel/Blueprint/Core/CombatSetup/BP_CombatSystem.BP_CombatSystem_C"))
  (Variables|Default|SetcombatSystem (Utilities|Array|Get(acopy) _outactors))
  (bind _outactors_2 (Actor|GetAllActorsOfClass "/Game/Development/MainGame/UnitSpawner.UnitSpawner_C"))
  (Variables|Default|SetspawnerRef (Utilities|Array|Get(acopy) _outactors_2))
  (bind _asgaming_instance (Utilities|Casting|CastToGamingInstance (Game|GetGameInstance)))
  (Variables|Default|SetNumb%20Of%20Players (Variables|/Game/Development/GamingInstance.GamingInstance_C|GetNumbOfPlayers _asgaming_instance))
  (bind _output_get (Variables|Default|SettimeRef (Variables|/Game/Development/GamingInstance.GamingInstance_C|GetSettetTurnTimer _asgaming_instance)))
  (Variables|Default|Settime _output_get)
  (CallFunction|SetPlayerCount _winmanager (Variables|/Game/Development/GamingInstance.GamingInstance_C|GetNumbOfPlayers _asgaming_instance))
  (CallFunction|SetMaxWin _winmanager (Variables|/Game/Development/GamingInstance.GamingInstance_C|GetSettetWinsNeeded _asgaming_instance)))

(fn SetPlayerActions
  (bind _outactors (Actor|GetAllActorsOfClass "/Game/Robin/NewLevel/Blueprint/Core/Player/BP_PlayerActions.BP_PlayerActions_C"))
  (Variables|Default|SetPlayerActions (Utilities|Array|Get(acopy) _outactors)))

(fn SetGamingInstance
  (bind _asgaming_instance (Utilities|Casting|CastToGamingInstance (Game|GetGameInstance)))
  (Variables|Default|SetAs%20Gaming%20Instance _asgaming_instance))

(fn SetTokenManager
  (bind _outactors (Actor|GetAllActorsOfClass 0))
  (Variables|Default|SettokenManager 0 0))

(fn SetCameraController
  (bind _outactors (Actor|GetAllActorsOfClass 0))
  (Variables|Default|SetcameraController 0 0))

(fn ResetUpPlayerUiifFailed
  (CallFunction|SetMaxPlayerIndex (.cameraController (Variables|Default|GetcameraController)) (Variables|Default|GetNumb%20Of%20Players))
  (bind _outactors (Actor|GetAllActorsOfClass 0))
  (Variables|Default|SettokenManager 0 0)
  (bind _foundwidgets (Widget|GetAllWidgetsOfClass "/Game/Development/UI/PlayerIndicator.PlayerIndicator_C" true))
  (Variables|Default|SetPlayerNumberUI (Utilities|Array|Get(acopy) _foundwidgets)))

(fn SetUpPlayerUi
  (bind _foundwidgets (Widget|GetAllWidgetsOfClass "/Game/Development/UI/PlayerIndicator.PlayerIndicator_C" false))
  (Variables|Default|SetPlayerNumberUI (Utilities|Array|Get(acopy) _foundwidgets))
  (bind _foundwidgets_2 (Widget|GetAllWidgetsOfClass "/Game/Development/MainGame/WB_startKingKiller.WB_startKingKiller_C" true))
  (Variables|Default|SetKingKillerWidget (Utilities|Array|Get(acopy) _foundwidgets_2))
  (return _foundwidgets))

(fn SetKingKilllerTokens
  (bind _numb_of_players (Variables|Default|GetNumb%20Of%20Players))
  (bind _as_gaming_instance (Variables|Default|GetAs%20Gaming%20Instance))
  (bind _kingkillerison (Variables|/Game/Development/GamingInstance.GamingInstance_C|GetKingKillerIsOn _as_gaming_instance))
  (if _kingkillerison
    (Variables|Default|SetKing%20Killer%20Is%20On _kingkillerison)
    (CallFunction|AddTokens (.tokenManager (Variables|Default|GettokenManager)) 1 _numb_of_players)
    (for _index (range 0 (- _numb_of_players 1))
      (CallFunction|GetTokens (.tokenManager (Variables|Default|GettokenManager)) _index))
    (Variables|Default|SetshowTxt true)))

(fn TurnTimer
  (CallFunction|Timer)
  (Default|ShowTimer (Variables|Default|GetPlayerNumberUI)))

(fn ResetDiceResults
  (bind _asbp_pc (Utilities|Casting|CastToBP_PC (Game|GetPlayerController 0)))
  (Variables|/Game/Robin/NewLevel/Blueprint/Core/Player/BP_PC.BP_PC_C|SetCanRoll _asbp_pc true)
  (bind _asbp_pc_2 (Utilities|Casting|CastToBP_PC (Game|GetPlayerController 0)))
  (Variables|/Game/Robin/NewLevel/Blueprint/Core/Player/BP_PC.BP_PC_C|SetResultPawnDice _asbp_pc_2 0)
  (Variables|/Game/Robin/NewLevel/Blueprint/Core/Player/BP_PC.BP_PC_C|SetResultUniversalDice _asbp_pc_2 0))

(fn ResetKingKillerTokenCheck
  (bind _kingkillerwidget (Variables|Default|GetKingKillerWidget))
  (Variables|/Game/Development/MainGame/WB_startKingKiller.WB_startKingKiller_C|SetsecomdPlayerCanChooese _kingkillerwidget true)
  (Variables|/Game/Development/MainGame/WB_startKingKiller.WB_startKingKiller_C|SetfirstPlayerDeniedKIngKiller _kingkillerwidget false))

(fn CheckWhichPlayerTurnItIs
  (params (A :type Integer) (A2 :type Integer) (A3 :type Integer))
  (if (== A2 1)
    (Variables|Default|SetshowTxt true)
    (Variables|Default|SetplayerTxt "Player 1")
    (elif (== A 2)
      (Variables|Default|SetshowTxt true)
      (Variables|Default|SetplayerTxt "Player2")
      (elif (== A3 3)
        (Variables|Default|SetshowTxt true)
        (Variables|Default|SetplayerTxt "Player 3")))))

(fn HandleUnitRespawn
  (bind _spawnerref (Variables|Default|GetspawnerRef))
  (bind _deadunits (Variables|/Game/Development/MainGame/UnitSpawner.UnitSpawner_C|GetdeadUnits _spawnerref))
  (LocalVariables|Setindex 0)
  (for _array_element (Variables|/Game/Development/MainGame/UnitSpawner.UnitSpawner_C|GetdeadUnits (Variables|Default|GetspawnerRef))
    (bind _returnvalue (CallFunction|GetPlayerID (.cameraController (Variables|Default|GetcameraController))))
    (if (== (Variables|/Game/Robin/NewLevel/Blueprint/Core/Units/BP_Unit.BP_Unit_C|GetTeamIndex _array_element) _returnvalue)
      (LocalVariables|SethasUnitsToRespawn true)))
  (if (LocalVariables|GethasUnitsToRespawn)
    (Audio|PlaySound2D "/Game/SoundDepartment/SFX/CooleSoundEffekt/SFX_Respawn.SFX_Respawn" 1.0 1.0 0.0 0 0)
    (bind (_arrayindex _arrayelement) (Utilities|Array|ReverseforEachLoop _deadunits)
      (:LoopBody
        (bind _output_get (Variables|Default|SetArray%20Element _arrayelement))
        (CallFunction|RespawnUnit _output_get (Utilities|Array|Get(acopy) _deadunits _arrayindex) _arrayindex)))))

(fn InitGame
  (bind _returnvalue (AddComponent|AddNiagaraComponent false))
  (bind _output_get (Variables|Default|SetVFX_RespawnGreen _returnvalue))
  (Components|Activation|Deactivate _output_get)
  (CallFunction|SetUpGameValues)
  (CallFunction|SetPlayerActions)
  (CallFunction|SetGamingInstance)
  (CallFunction|SetTokenManager)
  (CallFunction|SetCameraController)
  (bind _foundwidgets (CallFunction|SetUpPlayerUi))
  (return _foundwidgets))

(fn CheckifUnitIsonTile
  (params (spawnPoint :type Int%20Point%20Structure))
  (bind _spawnerref (Variables|Default|GetspawnerRef))
  (bind _playeractions (Variables|/Game/Robin/NewLevel/Blueprint/Core/Player/Actions/BP_Action.BP_Action_C|GetPlayerActions _spawnerref))
  (bind _grid (Variables|/Game/Robin/NewLevel/Blueprint/Core/Player/BP_PlayerActions.BP_PlayerActions_C|GetGrid _playeractions))
  (bind _gridtiles (Variables|/Game/Robin/NewLevel/Blueprint/Grid/BP_Grid.BP_Grid_C|GetGridTiles _grid))
  (bind _value (Utilities|Map|Find _gridtiles spawnPoint))
  (bind _unitontile (Utilities|Struct|BreakS_TileData _value))
  (Utilities|IsValid _unitontile
    (:Is%20Valid
      (Utilities|Array|Add (Variables|/Game/Development/MainGame/UnitSpawner.UnitSpawner_C|GetdeadUnits (Variables|Default|GetspawnerRef)) _unitontile)
      (bind _output_get (LocalVariables|SetUnitOnTile _unitontile))
      (bind _dummyunit (Default|SpawnDummyUnitwhenUnitNotValid (Variables|Default|GetcombatSystem) _output_get))
      (LocalVariables|Setdummyunit _dummyunit)
      (LocalVariables|SetindexRef (Variables|/Game/Robin/NewLevel/Blueprint/Core/Units/BP_Unit.BP_Unit_C|GetIndex (LocalVariables|GetUnitOnTile)))
      (Variables|/Game/Robin/NewLevel/Blueprint/Core/Units/BP_Unit.BP_Unit_C|SetIndex (LocalVariables|GetUnitOnTile) (Utilities|Struct|MakeIntPoint -999 -999))
      (Variables|/Game/Robin/NewLevel/Blueprint/Core/Units/BP_Unit.BP_Unit_C|SetisDead (LocalVariables|GetUnitOnTile) true)
      (Default|SetUnitIndexonGrid (Variables|Default|GetcombatSystem) (LocalVariables|GetUnitOnTile) (Variables|/Game/Robin/NewLevel/Blueprint/Core/Units/BP_Unit.BP_Unit_C|GetIndex (LocalVariables|GetUnitOnTile)) false true)
      (Default|SetUnitIndexonGrid (Variables|Default|GetcombatSystem) (LocalVariables|Getdummyunit) (LocalVariables|GetindexRef) true true)
      (Actor|DestroyActor (LocalVariables|Getdummyunit)))))

(fn HandleVFX
  (params (UnitTeamIndex :type Integer64) (Unit :type BP%20Unit%20Object%20Reference))
  (bind _spawnpos (Variables|/Game/Robin/NewLevel/Blueprint/Core/Units/BP_Unit.BP_Unit_C|GetSpawnPos Unit))
  (if (== UnitTeamIndex 1)
    (Game|SpawnActorfromClass "/Game/Art/VFX/BP_RespawnVFX.BP_RespawnVFX_C" (Math|Transform|MakeTransform _spawnpos "0, 0, 0" "1.000000,1.000000,1.000000") "Undefined" "MultiplyWithRoot" 0 0)
    (return)
    (elif (== UnitTeamIndex 2)
      (Game|SpawnActorfromClass "/Game/Art/VFX/BP_RspawnVFX_Pink.BP_RspawnVFX_Pink_C" (Math|Transform|MakeTransform _spawnpos "0, 0, 0" "1.000000,1.000000,1.000000") "Undefined" "MultiplyWithRoot" 0 0)
      (return)
      (elif (== UnitTeamIndex 3)
        (Game|SpawnActorfromClass "/Game/Art/VFX/BP_RespawnVFX_Blue.BP_RespawnVFX_Blue_C" (Math|Transform|MakeTransform _spawnpos "0, 0, 0" "1.000000,1.000000,1.000000") "Undefined" "MultiplyWithRoot" 0 0)
        (return)))))