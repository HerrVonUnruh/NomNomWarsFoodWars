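; Physics-driven die Blueprint that can be thrown with a random tumble.
; RollPawnDice randomizes the actor's rotation, teleports it to a fixed raised position and applies a very large random angular impulse to the Dice component.
; BeginPlay fills a side array with one to six, but no logic here reads it or detects the landed face.
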(event Custom|Roll%20Pawn%20Dice
  (Transformation|SetActorRotation (Math|Rotator|MakeRotator (Math|Random|RandomFloatinRange -1.8e+02 1.8e+02) (Math|Random|RandomFloatinRange -1.8e+02 1.8e+02) (Math|Random|RandomFloatinRange -1.8e+02 1.8e+02)))
  (Transformation|SetActorLocation (Math|Vector|MakeVector 0.0 0.0 2e+03) false false)
  (Class|PrimitiveComponent|AddAngularImpulseinDegrees (Variables|Default|Getdice) (Math|Vector|MakeVector (Math|Random|RandomFloatinRange 4e+08 5e+08) (Math|Random|RandomFloatinRange 4e+08 5e+08) (Math|Random|RandomFloatinRange 4e+08 5e+08)) "None" false))

(event EventBeginPlay
  (Variables|Default|SetpSideArr (Utilities|Array|MakeArray (Variables|Default|Get1) (Variables|Default|Get2) (Variables|Default|Get3) (Variables|Default|Get4) (Variables|Default|Get5) (Variables|Default|Get6))))

(event Collision|EventActorBeginOverlap
  (params (OtherActor :type Actor%20Object%20Reference)))

(event EventTick
  (params (DeltaSeconds :type Float%20%28single-precision%29)))

(fn ConstructionScript)