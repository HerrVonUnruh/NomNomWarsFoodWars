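; Simple enemy Blueprint for an FPS that chases the player and dies when shot.
; On BeginPlay it caches the BP_FPSCharachter actor, then reissues AIMoveTo to that actor's current location every Tick.
; Each overlap with an actor of class BP_Bullet subtracts fixed Health and prints a hit message.
; Tick also polls Health and destroys the enemy at zero or below instead of moving it.
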(event EventBeginPlay
  (bind _returnvalue (Actor|GetActorOfClass "/Game/Development/FPS/BP_FPSCharachter.BP_FPSCharachter_C"))
  (Variables|Default|SetPlayer _returnvalue))

(event Collision|EventActorBeginOverlap
  (params (OtherActor :type Actor%20Object%20Reference))
  (if (== (Utilities|GetClass OtherActor) "/Game/Development/FPS/BP_Bullet.BP_Bullet_C")
    (Variables|Default|SetHealth (- (Variables|Default|GetHealth) 5.0))
    (Development|PrintText "enemy hit")))

(event EventTick
  (params (DeltaSeconds :type Float%20%28single-precision%29))
  (if (<= (Variables|Default|GetHealth) 0.0)
    (Actor|DestroyActor)
    (else
      (AI|AIMoveTo 0 (Transformation|GetActorLocation (Variables|Default|GetPlayer)) 0 -1.0 "Default" "Default" true true))))

(fn ConstructionScript)