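; BP_FPSEnemy is an FPS enemy that creeps toward the player, takes damage from bullets and hurts the player on overlap.
; BeginPlay caches the first BP_FPSCharachter and BP_KingKillerTimer in the level.
; Overlapping bullets reduce Health and are destroyed, while overlapping the player calls its TakeDamage.
; While the timer is above zero, Tick lerps position toward the player without sweep at a frame-rate-dependent rate, or at zero Health decrements the player's EnemyCount and destroys itself.
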(event EventBeginPlay
  (bind _returnvalue (Actor|GetActorOfClass "/Game/Development/FPS/BP_FPSCharachter.BP_FPSCharachter_C"))
  (Variables|Default|SetPlayer _returnvalue)
  (bind _returnvalue_2 (Actor|GetActorOfClass "/Game/Development/FPS/BP_KingKillerTimer.BP_KingKillerTimer_C"))
  (Variables|Default|Settimer _returnvalue_2))

(event Collision|EventActorBeginOverlap
  (params (OtherActor :type Actor%20Object%20Reference))
  (bind _returnvalue (Utilities|GetClass OtherActor))
  (if (== _returnvalue "/Game/Development/FPS/BP_Bullet.BP_Bullet_C")
    (Variables|Default|SetHealth (- (Variables|Default|GetHealth) 5.0))
    (Development|PrintText "enemy hit")
    (Actor|DestroyActor OtherActor)
    (elif (== _returnvalue "/Game/Development/FPS/BP_FPSCharachter.BP_FPSCharachter_C")
      (Class|SkriptFPSCharachter|TakeDamage (Variables|Default|GetPlayer)))))

(event EventTick
  (params (DeltaSeconds :type Float%20%28single-precision%29))
  (bind _returnvalue (Class|SkriptKingKillerTimer|GetTimerValue (Variables|Default|Gettimer)))
  (if (not (<= _returnvalue 0.0))
    (if (<= (Variables|Default|GetHealth) 0.0)
      (Variables|/Game/Development/FPS/BP_FPSCharachter.BP_FPSCharachter_C|SetEnemyCount (Variables|Default|GetPlayer) (- (Variables|/Game/Development/FPS/BP_FPSCharachter.BP_FPSCharachter_C|GetEnemyCount (Variables|Default|GetPlayer)) 1))
      (Actor|DestroyActor)
      (else
        (Transformation|SetActorLocation (Math|Vector|Lerp(Vector) (Transformation|GetActorLocation) (Transformation|GetActorLocation (Variables|Default|GetPlayer)) 0.0025) false false)))))

(fn ConstructionScript)