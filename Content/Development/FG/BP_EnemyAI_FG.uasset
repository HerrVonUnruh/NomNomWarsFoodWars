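; Enemy AI Blueprint in an FG development folder that moves toward the player and turns to face it.
; BeginPlay caches the first BP_FGPlayer, which the AI_Movement event uses as the AIMoveTo target and for a yaw-only look-at rotation.
; AI_Movement is not called within this graph.
; The box collider overlap only runs a DoOnce with a short delayed reset, with no gameplay action attached.
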(event OnComponentBeginOverlap(Box_Collider)
  (params (OverlappedComponent :type Primitive%20Component%20Object%20Reference) (OtherActor :type Actor%20Object%20Reference) (OtherComp :type Primitive%20Component%20Object%20Reference) (OtherBodyIndex :type Integer) (bFromSweep :type Boolean) (SweepResult :type Hit%20Result%20Structure%20%28by%20ref%29))
  (Utilities|FlowControl|DoOnce false :!label _label
    (:Completed
      (Utilities|FlowControl|Delay 0.2)
      (goto _label Reset))))

(event Custom|AI_Movement
  (bind _self self)
  (AI|AIMoveTo _self "0, 0, 0" (Variables|Default|GetPlayer_Ref) 1e+02 false
    (:then
      (Transformation|SetActorRotation (Math|Rotator|MakeRotator 0.0 0.0 (.yaw (Math|Rotator|FindLookatRotation (.location (Transformation|GetActorTransform _self)) (.location (Transformation|GetActorTransform (Variables|Default|GetPlayer_Ref))))))))))

(event EventBeginPlay
  (bind _outactors (Actor|GetAllActorsOfClass "/Game/Development/FG/BP_FGPlayer.BP_FGPlayer_C"))
  (Variables|Default|SetPlayer_Ref (Utilities|Array|Get(acopy) _outactors)))

(event Collision|EventActorBeginOverlap
  (params (OtherActor :type Actor%20Object%20Reference)))

(event EventTick
  (params (DeltaSeconds :type Float%20%28single-precision%29)))

(fn ConstructionScript)