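; GM_FG is a game mode Blueprint, apparently for a fighting game, that is mostly a skeleton.
; BeginPlay and the construction script only call their parent versions.
; The DisplayCharacterSelecet and Spawn Player functions contain no logic and just return false.
; Unconnected EventGraph nodes would fetch a TestFighter actor and set the first player's controller ID, but never run.
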(event EventBeginPlay
  (|CallParentFunction))

(fn ConstructionScript
  (|CallParentFunction))

(fn DisplayCharacterSelecet
  (params (PlayerIndex :type Integer))
  (return false))

(fn SpawnPlayer
  (params (CurrentPlayerIndex :type Integer) (InputReceiver :type BP%20Input%20Receiver%20Object%20Reference))
  (return false))